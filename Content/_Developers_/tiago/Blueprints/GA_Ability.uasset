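; GA_Ability is a Gameplay Ability that spawns a trap in front of the third-person character.
; On activation it casts the avatar to BP_ThirdPersonCharacter and offsets the movement component's last update location by a fixed vector rotated with the full camera rotation, so pitch affects placement.
; It spawns the actor unrotated, prints a debug message and ends immediately, with no commit step.
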(event Ability|EventActivateAbility
  ;[0.05 0.05 0.05] Trap Spawn Logic
  (bind _asbp_third_person_character (Utilities|Casting|CastToBP_ThirdPersonCharacter (Ability|GetAvatarActorfromActorInfo)))
  (Game|SpawnActorfromClass "/Game/_Developers_/tiago/Blueprints/BP_Trap.BP_Trap_C" (Math|Transform|MakeTransform (+ (Class|CharacterMovementComponent|GetLastUpdateLocation (Variables|/Script/Engine.Character|GetCharacterMovement _asbp_third_person_character)) (Math|Vector|RotateVector "150.000000,0.000000,10.000000" (Camera|GetCameraRotation (Game|GetPlayerCameraManager 0))))) "Undefined" "OverrideRootScale" 0 0)
  (Development|PrintString "Spawned Trap!")
  (Ability|EndAbility))